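; BP_Item_01 is a pickup item actor that shows an on-screen pickup prompt while the ThirdPersonCharacter is in range.
; Entering its Box trigger creates a WG_PickupText widget, stores it and adds it to the viewport; leaving removes it.
; The CustomInterfacePickup event removes the prompt and destroys the actor, with no inventory or reward logic in this Blueprint.
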(event `self.Box.OnComponentBeginOverlap`
  (params (OverlappedComponent :type "PrimitiveComponent Object Reference") (OtherActor :type "Actor Object Reference") (OtherComp :type "PrimitiveComponent Object Reference") (OtherBodyIndex :type Integer) (bFromSweep :type Boolean) (SweepResult :type "HitResult Structure (by ref)"))
  (cast `/Game/ThirdPersonBP/Blueprints/ThirdPersonCharacter` OtherActor)
  (bind _returnvalue (`|CreateWidget` "/Game/AIG/UI/WG_PickupText.WG_PickupText_C"))
  (bind _output_get (set `self.PickupTextWigetRef` _returnvalue))
  (`UserWidget.AddToViewport` _output_get 0))

(event `self.Box.OnComponentEndOverlap`
  (params (OverlappedComponent :type "PrimitiveComponent Object Reference") (OtherActor :type "Actor Object Reference") (OtherComp :type "PrimitiveComponent Object Reference") (OtherBodyIndex :type Integer))
  (cast `/Game/ThirdPersonBP/Blueprints/ThirdPersonCharacter` OtherActor)
  (`Widget.RemoveFromParent` (`self.PickupTextWigetRef`)))

(event `/Game/AIG/Blueprint/Interface/BI_PickupItems.CustomInterfacePickup`
  (`Widget.RemoveFromParent` (`self.PickupTextWigetRef`))
  (`self.K2_DestroyActor`))

(fn `UserConstructionScript`)