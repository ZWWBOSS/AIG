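; Level exit trigger actor that opens Level_02_Persistent when the ThirdPersonCharacter overlaps it.
; On overlap it fades the camera to black, waits a second, then loads the level by name, a step marked as test only.
; BeginPlay caches the player's start transform, used only by disconnected logic that would gate the exit on remaining BI_PickupItems actors and otherwise teleport the player back near the start.
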(event `self.ReceiveBeginPlay`
  (bind _asthird_person_character (cast `/Game/ThirdPersonBP/Blueprints/ThirdPersonCharacter` (`GameplayStatics.GetPlayerCharacter` 0)))
  (set `self.StartLocation` (`self.K2_GetActorLocation` _asthird_person_character))
  (set `self.StartRotation` (`self.K2_GetActorRotation` _asthird_person_character)))

(event `self.ReceiveActorBeginOverlap`
  (params (OtherActor :type "Actor Object Reference"))
  (cast `/Game/ThirdPersonBP/Blueprints/ThirdPersonCharacter` OtherActor)
  (`PlayerCameraManager.StartCameraFade` :`self` (`GameplayStatics.GetPlayerCameraManager` 0) :`ToAlpha` 1.0 :`Duration` 1.0 :`bHoldWhenFinished` true)
  (`KismetSystemLibrary.Delay` 1.0)
  ;[1 1 1] Test Only
  (`GameplayStatics.OpenLevel` "Level_02_Persistent"))

(fn `UserConstructionScript`)